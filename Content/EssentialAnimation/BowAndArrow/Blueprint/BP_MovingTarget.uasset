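; BP_MovingTarget is a shooting target that shuttles between two points and awards score when hit.
; Tick moves the MovingTarget component toward TargetPoint01 or TargetPoint02 at Speed, flipping IsMovingToA within a small threshold.
; The world-space direction is applied through AddLocalOffset, so component rotation affects the path.
; The Hit event briefly swaps to a highlight material and increments Score on the player's BP_ThirdPersonCharacter.
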(event `self.ReceiveTick`
  (params (DeltaSeconds :type "Float (single-precision)"))
  (bind _moving_target (`self.Moving_Target`))
  (bind _returnvalue (`SceneComponent.K2_GetComponentLocation` _moving_target))
  (bind _returnvalue_2 (- (`SceneComponent.K2_GetComponentLocation` (`self.Target_Point_01`)) _returnvalue))
  (bind _returnvalue_3 (- (`SceneComponent.K2_GetComponentLocation` (`self.Target_Point_02`)) _returnvalue))
  (if (`self.isMovingToA`)
    (`SceneComponent.K2_AddLocalOffset` _moving_target (* (`KismetMathLibrary.Normal` _returnvalue_2) (* (`self.speed`) DeltaSeconds)) false false)
    (if (< (`KismetMathLibrary.VSize` _returnvalue_2) 5.0)
      (set `self.isMovingToA` false))
    (else
      (`SceneComponent.K2_AddLocalOffset` _moving_target (* (`KismetMathLibrary.Normal` _returnvalue_3) (* (`self.speed`) DeltaSeconds)) false false)
      (if (< (`KismetMathLibrary.VSize` _returnvalue_3) 5.0)
        (set `self.isMovingToA` true)))))

(event `Hit`
  (`PrimitiveComponent.SetMaterial` (`self.Moving_Target`) 0 "/Game/EssentialAnimation/BowAndArrow/Demo/Material/MI_Hitbox_Light.MI_Hitbox_Light")
  (bind _asbp_third_person_character (cast `/Game/EssentialAnimation/BowAndArrow/Blueprint/BP_ThirdPersonCharacter` (`GameplayStatics.GetPlayerPawn` 0)))
  (`/Engine/EditorBlueprintResources/StandardMacros.IncrementInt` (`/Game/EssentialAnimation/BowAndArrow/Blueprint/BP_ThirdPersonCharacter.score` _asbp_third_person_character)
    (:`  `
      (`KismetSystemLibrary.Delay` 0.2)
      (`PrimitiveComponent.SetMaterial` (`self.Moving_Target`) 0 "/Game/EssentialAnimation/BowAndArrow/Demo/Material/MI_ShootingTarget.MI_ShootingTarget"))))

(fn `UserConstructionScript`)