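; Physics-driven arrow projectile for a bow, with a particle trail and optional timed self-destruction.
; SetVelocity launches the mesh along a given direction at a given force.
; On overlap it ends the trail and notifies any BP_MovingTarget of the hit.
; For anything except the third-person character, it spawns a burst and a static arrow copy, knocks movable overlapping components away and attaches the copy to them.
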(event `self.ReceiveBeginPlay`
  (bind _trail (`self.Trail`))
  (`ActorComponent.Activate` _trail false)
  (`ParticleSystemComponent.BeginTrails` _trail "Trail_01" "Trail_02" "ETrailWidthMode_FromFirst" 2.0)
  (if (`self.isAutoSelfDestroy`)
    (`KismetSystemLibrary.Delay` 5.0)
    (`self.K2_DestroyActor`)))

(event `SetVelocity`
  (params (ForceLength :type "Float (double-precision)") (Velocity :type "Vector Structure"))
  (`PrimitiveComponent.SetPhysicsLinearVelocity` (`self.Mesh`) (* (`KismetMathLibrary.Normal` Velocity) ForceLength) true "None"))

(event `self.ReceiveActorBeginOverlap`
  (params (OtherActor :type "Actor Object Reference"))
  (bind _returnvalue (`SceneComponent.K2_GetComponentToWorld` (`self.Mesh`)))
  (`ParticleSystemComponent.EndTrails` (`self.Trail`))
  (bind _asbp_moving_target (cast `/Game/EssentialAnimation/BowAndArrow/Blueprint/BP_MovingTarget` OtherActor)
    (:`then`
      (`/Game/EssentialAnimation/BowAndArrow/Blueprint/BP_MovingTarget.Hit` _asbp_moving_target))
    (:`CastFailed`
      _))
  (if (!= (`GameplayStatics.GetObjectClass` OtherActor) "/Game/EssentialAnimation/BowAndArrow/Blueprint/BP_ThirdPersonCharacter.BP_ThirdPersonCharacter_C")
    (`KismetSystemLibrary.PrintString` "Hit")
    (bind _returnvalue_2 (`|SpawnActorFromClass` "/Script/Engine.StaticMeshActor" _returnvalue "Undefined" "MultiplyWithRoot" null null))
    (`StaticMeshActor.SetMobility` _returnvalue_2 "Movable")
    (`StaticMeshComponent.SetStaticMesh` (`StaticMeshActor.StaticMeshComponent` _returnvalue_2) "/Game/Project_X/Character/Weapon/SM_Arrow.SM_Arrow")
    (`GameplayStatics.SpawnEmitterAtLocation` "/Game/EssentialAnimation/BowAndArrow/Demo/Particles/P_HitBurst.P_HitBurst" (.location _returnvalue) (struct) (0.5 0.5 0.5))
    (for _array_element (`PrimitiveComponent.GetOverlappingComponents` (`self.Mesh`))
      (if (`|EnumEquality` (`SceneComponent.Mobility` _array_element) "Movable")
        (`PrimitiveComponent.SetPhysicsLinearVelocity` _array_element (* (`KismetMathLibrary.Normal` (- (`self.K2_GetActorLocation` OtherActor) (`SceneComponent.K2_GetComponentLocation` (`self.Mesh`)))) 2000.0) false "None")
        (`SceneComponent.K2_AttachToComponent` (`Actor.RootComponent` _returnvalue_2) _array_element "None" "KeepRelative" "KeepRelative" "KeepRelative" true)))))

(fn `UserConstructionScript`)