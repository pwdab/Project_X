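; Bow item actor for Project_X that displays itself with a spinning, bobbing idle animation.
; On BeginPlay, only non-authority instances start a timeline that turns the actor's yaw at a fixed roll tilt.
; Each update of that timeline stores the actor location and calls Play on a second timeline.
; That timeline sets the Mesh's relative location from the stored actor location plus a sine-wave Z offset.
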(event `self.ReceiveBeginPlay`
  (bind (_baselocation_x _baselocation_y _baselocation_z) (`KismetMathLibrary.BreakVector` (`self.BaseLocation`)))
  (`/Engine/EditorBlueprintResources/ActorMacros.Switch Has Authority`
    (:`Remote`
      (bind (_direction `_새_트랙_0`) (`Timeline|타임라인`)
        (:`Update`
          (`self.K2_SetActorRotation` (`KismetMathLibrary.MakeRotator` -30.0 0.0 `_새_트랙_0`))
          (set `self.BaseLocation` (`self.K2_GetActorLocation`))
          (bind (_direction_2 `_새_트랙_0_2`) (`Timeline|타임라인_0`)
            (:`Update`
              (`SceneComponent.K2_SetRelativeLocation` (`self.Mesh`) (`KismetMathLibrary.MakeVector` _baselocation_x _baselocation_y (+ _baselocation_z (* (`KismetMathLibrary.Sin` (`KismetMathLibrary.MultiplyByPi` (* `_새_트랙_0_2` 2.0))) (`self.Multiply`)))) false false))))))))

(fn `UserConstructionScript`)